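; BP_NPC is an NPC pawn that patrols a looping route while its mesh bobs up and down.
; On BeginPlay it records the mesh's starting height, then chains AI MoveTo calls through the PatrolPoints array, wrapping to the first after the last and advancing only on success.
; Each tick it offsets the mesh vertically by FloatSpeed, flipping direction at MaxFloatOffset from that height, without delta-time scaling.
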(event EventBeginPlay
  (bind _patrolpoints (Variables|Default|GetPatrolPoints))
  (Variables|Default|SetDefaultZ (.z (Variables|/Script/Engine.SceneComponent|GetRelativeLocation (Variables|Character|GetMesh))))
  ;[1 1 1] Patrolling
  (AI|AIMoveTo self (Utilities|Array|Get(acopy) _patrolpoints (Variables|Default|GetPatrolNumber)) 0 5.0 false :!label _label
    (:OnSuccess
      (if (> (+ (Variables|Default|GetPatrolNumber) 1) (Utilities|Array|LastIndex _patrolpoints))
        (Variables|Default|SetPatrolNumber 0)
        (goto _label)
        (else
          (Variables|Default|SetPatrolNumber (+ (Variables|Default|GetPatrolNumber) 1))
          (goto _label))))))

(event EventTick
  (params (DeltaSeconds :type Float%20%28single-precision%29))
  (bind _mesh (Variables|Character|GetMesh))
  ;[1 1 1] Floating
  (Transformation|AddLocalOffset _mesh (Math|Vector|MakeVector 0.0 0.0 (* (Variables|Default|GetFloatSpeed) (Math|Integer|SelectInt 1 -1 (Variables|Default|GetFloatUp)))) false false)
  (if (>= (Math|Float|Absolute(Float) (- (.z (Variables|/Script/Engine.SceneComponent|GetRelativeLocation _mesh)) (Variables|Default|GetDefaultZ))) (Variables|Default|GetMaxFloatOffset))
    (Variables|Default|SetFloatUp (not (Variables|Default|GetFloatUp)))))

(fn ConstructionScript)