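; BP_DinoArmCollider is a collider, apparently for a dinosaur arm, that picks up and drops BP_Pickup objects.
; Begin and end overlaps track a single candidate pickup while nothing is held, toggling the player HUD's pickup prompt.
; The PickUpObject event attaches that candidate to the Collider with physics disabled, or detaches the held object and re-enables its physics.
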(event Custom|Pick%20Up%20Object
  (if (Utilities|IsValid (Variables|Default|GetHolding))
    ;[1 1 1] Drop Object
    (Transformation|DetachFromActor (Variables|Default|GetHolding) "KeepWorld" "KeepRelative" "KeepRelative")
    (bind _asbp_pickup (Utilities|Casting|CastToBP_Pickup (Variables|Default|GetHolding)))
    (Default|TogglePhysics _asbp_pickup true)
    (Variables|Default|SetHolding 0)
    (Variables|Default|SetOverlapping 0)
    (else
      ;[1 1 1] Pick Up Object
      (if (Utilities|IsValid (Variables|Default|GetOverlapping))
        (bind _asbp_pickup_2 (Utilities|Casting|CastToBP_Pickup (Variables|Default|GetOverlapping)))
        (Default|TogglePhysics _asbp_pickup_2 false)
        (Transformation|AttachComponentToComponent (Variables|Default|GetOverlapping) (Variables|Default|GetCollider) "None" "KeepWorld" "KeepRelative" "KeepWorld" true)
        (Variables|Default|SetHolding (Variables|Default|GetOverlapping))
        (Variables|Default|SetOverlapping 0)
        (Default|TogglePickupText (Variables|/Game/ThirdPerson/Blueprints/BP_ThirdPersonCharacter.BP_ThirdPersonCharacter_C|GetHUD (Variables|Default|GetPlayer)) false)))))

(event Collision|EventActorBeginOverlap
  (params (OtherActor :type Actor%20Object%20Reference))
  ;[1 1 1] Collision Detection
  (if (and (Utilities|ClassIsChildOf (Utilities|GetClass OtherActor) "/Game/Blueprints/BP_Pickup.BP_Pickup_C") (and (not (Utilities|IsValid (Variables|Default|GetOverlapping))) (not (Utilities|IsValid (Variables|Default|GetHolding)))))
    (Variables|Default|SetOverlapping OtherActor)
    (Default|TogglePickupText (Variables|/Game/ThirdPerson/Blueprints/BP_ThirdPersonCharacter.BP_ThirdPersonCharacter_C|GetHUD (Variables|Default|GetPlayer)) (Utilities|IsValid (Variables|Default|GetOverlapping)))))

(event Collision|EventActorEndOverlap
  (params (OtherActor :type Actor%20Object%20Reference))
  ;[1 1 1] Collision Detection
  (if (and (Utilities|ClassIsChildOf (Utilities|GetClass OtherActor) "/Game/Blueprints/BP_Pickup.BP_Pickup_C") (and (Utilities|IsValid (Variables|Default|GetOverlapping)) (not (Utilities|IsValid (Variables|Default|GetHolding)))))
    (Variables|Default|SetOverlapping 0)
    (Default|TogglePickupText (Variables|/Game/ThirdPerson/Blueprints/BP_ThirdPersonCharacter.BP_ThirdPersonCharacter_C|GetHUD (Variables|Default|GetPlayer)) (Utilities|IsValid (Variables|Default|GetOverlapping)))))

(event EventBeginPlay
  ;[1 1 1] Initialize Variables
  (bind _asbp_third_person_character (Utilities|Casting|CastToBP_ThirdPersonCharacter (Game|GetPlayerCharacter 0)))
  (Variables|Default|SetPlayer _asbp_third_person_character))

(fn ConstructionScript)